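; BP_Altar is a ritual altar actor that advances the game flow once its ritual effect is active.
; ActivateRitualFX swaps the magic circle decal for a Niagara effect and marks the altar active.
; When AltarTrigger registers an overlap on an active altar, it waits two seconds, then sets a new flow state on BP_GameMode, with no check on which actor entered.
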(event OnComponentBeginOverlap(AltarTrigger)
  (params (OverlappedComponent :type Primitive%20Component%20Object%20Reference) (OtherActor :type Actor%20Object%20Reference) (OtherComp :type Primitive%20Component%20Object%20Reference) (OtherBodyIndex :type Integer) (bFromSweep :type Boolean) (SweepResult :type Hit%20Result%20Structure%20%28by%20ref%29))
  (if (Variables|Default|GetbAltarActive)
    (Utilities|FlowControl|Delay 2.0)
    (bind _asbp_game_mode (Utilities|Casting|CastToBP_GameMode (Game|GetGameMode)))
    (Default|SetFlowState _asbp_game_mode "NewEnumerator3")))

(event Custom|ActivateRitualFX
  (bind _magiccircleniagara (Variables|Default|GetMagicCircleNiagara))
  (Rendering|SetVisibility (Variables|Default|GetMagicCircleDecal) false false)
  (Rendering|SetVisibility _magiccircleniagara true false)
  (Components|Activation|Activate _magiccircleniagara false)
  (Variables|Default|SetbAltarActive true))

(fn ConstructionScript)