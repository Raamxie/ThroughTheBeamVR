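; AI controller for the Stalker monster, which tracks the VR player and is meant to flee flashlight light.
; It runs BT_Stalker and feeds perception updates into blackboard target, last-known location and sight keys.
; A looping timer tests the pawn against the flashlight's range, cone and line trace before setting bShouldFlee.
; That trace ignores the pawn yet requires hitting it, so the flee check cannot pass as written.
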(event OnTargetPerceptionUpdated(AIPerception)
  (params (Actor :type Actor%20Object%20Reference) (Stimulus :type AI%20Stimulus%20Structure))
  (bind (_age _expirationage _strength _stimuluslocation _receiverlocation _tag _bsuccessfullysensed) (Utilities|Struct|BreakAIStimulus Stimulus))
  (bind _blackboard (Variables|Default|GetBlackboard))
  (bind _blackboard_2 (Variables|Default|GetBlackboard))
  (Utilities|FlowControl|Delay 0.1)
  (bind _asbp_xrpawn (Utilities|Casting|CastToBP_XRPawn Actor))
  (bind _returnvalue (Class|AIPerceptionSystem|GetSenseClassforStimulus Stimulus))
  (if _bsuccessfullysensed
    (AI|Components|Blackboard|SetValueasObject _blackboard_2 (Utilities|Name|MakeLiteralName "TargetActor") _asbp_xrpawn)
    (AI|Components|Blackboard|SetValueasVector _blackboard_2 (Utilities|Name|MakeLiteralName "LastKnownLocation") _stimuluslocation)
    (AI|Components|Blackboard|SetValueasBool _blackboard_2 (Utilities|Name|MakeLiteralName "bHasLastKnown") true)
    (if (== _returnvalue "/Script/AIModule.AISenseConfig_Sight")
      (AI|Components|Blackboard|SetValueasBool _blackboard (Utilities|Name|MakeLiteralName "bCanSeePlayer") true)
      (else
        (AI|Components|Blackboard|SetValueasBool _blackboard (Utilities|Name|MakeLiteralName "bCanSeePlayer") false)))
    (else
      (AI|Components|Blackboard|SetValueasBool _blackboard_2 (Utilities|Name|MakeLiteralName "bCanSeePlayer") false)
      (AI|Components|Blackboard|SetValueasObject _blackboard_2 (Utilities|Name|MakeLiteralName "TargetActor") 0))))

(event Custom|CheckFlashlight
  (bind _returnvalue (Pawn|GetControlledPawn))
  (bind _returnvalue_2 (Pawn|GetControlledPawn))
  (bind _spotref (Variables|Default|GetSpotRef))
  (bind _spotref_2 (Variables|Default|GetSpotRef))
  (bind _blackboard (Variables|Default|GetBlackboard))
  (bind _returnvalue_3 (Transformation|GetActorLocation _returnvalue_2))
  (bind _returnvalue_4 (Transformation|GetWorldLocation _spotref))
  (bind _returnvalue_5 (- _returnvalue_3 _returnvalue_4))
  (Variables|Default|SetMonsterLoc _returnvalue_3)
  (if (< (Math|Vector|VectorLength _returnvalue_5) 2.5e+03)
    (if (>= (Math|Vector|DotProduct (Math|Vector|GetForwardVector _spotref_2) (Math|Vector|Normalize _returnvalue_5)) (Math|Trig|Cos(Degrees) (* (Variables|/Script/Engine.SpotLightComponent|GetOuterConeAngle _spotref_2) 0.5)))
      (bind _outhit (Collision|LineTraceByChannel (Transformation|GetWorldLocation (Variables|Default|GetSpotRef)) (Variables|Default|GetMonsterLoc) "TraceTypeQuery1" false (Utilities|Array|MakeArray (Variables|Default|GetFlashlightRef) _returnvalue) "None"))
      (if (== (.hitactor _outhit) _returnvalue)
        (if (not (ScalableFloat|GetValueasBool (Variables|Default|GetBlackboard) (Utilities|Name|MakeLiteralName "bShouldFlee")))
          (bind _asbp_xrpawn (Utilities|Casting|CastToBP_XRPawn (Game|Player|GetPlayerPawn 0)))
          (AI|Components|Blackboard|SetValueasObject _blackboard (Utilities|Name|MakeLiteralName "TargetActor") _asbp_xrpawn)
          (AI|Components|Blackboard|SetValueasBool _blackboard (Utilities|Name|MakeLiteralName "bShouldFlee") true))))))

(event EventBeginPlay
  (bind _returnvalue (Actor|GetActorOfClass "/Game/Objects/Flashlight/Flashlight.Flashlight_C"))
  (bind _asflashlight (Utilities|Casting|CastToFlashlight _returnvalue))
  (bind _output_get (Variables|Default|SetFlashlightRef _asflashlight))
  (Variables|Default|SetSpotRef (Variables|/Game/Objects/Flashlight/Flashlight.Flashlight_C|GetSpotLight _output_get))
  (Utilities|Time|SetTimerbyEvent (delegate Custom|CheckFlashlight) 0.1 true))

(event EventPossess
  (params (PossessedPawn :type Pawn%20Object%20Reference))
  (Utilities|FlowControl|Delay 0.1)
  (AI|RunBehaviorTree "/Game/Emu/AI/BT_Stalker.BT_Stalker"))

(fn ConstructionScript)