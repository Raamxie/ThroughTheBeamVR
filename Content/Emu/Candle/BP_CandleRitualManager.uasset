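; Manager for an ordered candle-lighting puzzle that reports a checkpoint to BP_GameMode when solved.
; Each lighting attempt lights the candle and compares its Index with the expected CurrentIndex, advancing on a match.
; A wrong candle stays lit for a short delay before all candles are extinguished and progress resets.
; Completing the sequence sets Completed, blocking further attempts, and notifies the game mode.
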(event Custom|TryLightCandle
  (params (Candle :type BP%20Candle%20Object%20Reference))
  (if (not (Variables|Default|GetbCompleted))
    (if (Utilities|IsValid Candle)
      (Default|SetLit Candle true)
      (if (== (Variables|/Game/Emu/Candle/BP_Candle.BP_Candle_C|GetIndex Candle) (Variables|Default|GetCurrentIndex))
        (bind _output_get (Variables|Default|SetCurrentIndex (+ (Variables|Default|GetCurrentIndex) 1)))
        (if (>= _output_get (Utilities|Array|Length (Variables|Default|GetCandles)))
          (CallFunction|CompletePuzzle))
        (else
          (Utilities|FlowControl|Delay 2.0)
          (CallFunction|ResetPuzzle))))))

(event Custom|ResetPuzzle
  (for _array_element (Variables|Default|GetCandles)
    (Default|SetLit _array_element false))
  (Variables|Default|SetCurrentIndex 0))

(event Custom|CompletePuzzle
  (Variables|Default|SetbCompleted true)
  (bind _asbp_game_mode (Utilities|Casting|CastToBP_GameMode (Game|GetGameMode)))
  (Default|NotifyCheckpointCompleted _asbp_game_mode "NewEnumerator0"))

(fn ConstructionScript)