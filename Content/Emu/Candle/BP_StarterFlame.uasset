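; Configurable candle prop whose construction script builds its look from exposed settings; it has no runtime logic.
; ApplyCandleSettings toggles and tunes flame VFX, smoke, point light and crackle audio, which starts at a random offset.
; The mesh comes from CandleType or a position-seeded random stream, and also sets flame placement and wick burn height.
; Wax uses preset or custom-color materials, while a lit wick gets a dynamic emissive material.
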(event EventBeginPlay)

(fn ConstructionScript
  (CallFunction|ApplyCandleSettings))

(fn ApplyCandleSettings
  (bind _returnvalue (Transformation|GetActorLocation))
  (bind _candle (Variables|Default|GetCandle))
  (bind _candle_2 (Variables|Default|GetCandle))
  (bind _candleflame (Variables|Default|GetCandleFlame))
  (bind _pointlight (Variables|Default|GetPointLight))
  (bind _candle_3 (Variables|Default|GetCandle))
  (bind _flame_position (Variables|Default|GetFlame%20Position))
  (bind _sfx_vefects_candle_crackling_loop_01_randomized_cue (Variables|Default|GetSFX_Vefects_Candle_Crackling_Loop_01_Randomized_Cue))
  (bind _smokeloop (Variables|Default|GetSmokeLoop))
  (bind (_x _y _z) (Math|Vector|BreakVector _returnvalue))
  (Niagara|SetNiagaraVariable(Float) (Variables|Default|GetCandleFlame) "Size" (Variables|Default|GetFlame%20Size))
  (Niagara|SetNiagaraVariable(LinearColor) (Variables|Default|GetCandleFlame) "Color 01" (Variables|Default|GetFlame%20Color))
  (if (Variables|Default|GetFlame)
    (Components|Activation|SetAutoActivate _sfx_vefects_candle_crackling_loop_01_randomized_cue true)
    (Audio|Components|Audio|Play _sfx_vefects_candle_crackling_loop_01_randomized_cue (Math|Random|RandomFloatinRange 0.0 22.0))
    (else
      (Components|Activation|SetAutoActivate _sfx_vefects_candle_crackling_loop_01_randomized_cue false)))
  (if (Variables|Default|GetFlame)
    (Components|Activation|SetAutoActivate _candleflame true)
    (Effects|Components|ParticleSystem|SetBoolParameter _candleflame "CandleVertical" (Variables|Default|GetFlame%20Vertical))
    (else
      (Components|Activation|SetAutoActivate _candleflame false)))
  (if (Variables|Default|GetSmoke)
    (Components|Activation|SetAutoActivate _smokeloop true)
    (else
      (Components|Activation|SetAutoActivate _smokeloop false)))
  (if (Variables|Default|GetLight)
    (Rendering|SetVisibility _pointlight true false)
    (Development|SetHiddeninGame _pointlight false false)
    (else
      (Rendering|SetVisibility _pointlight false false)
      (Development|SetHiddeninGame _pointlight true false)))
  (Rendering|Components|Light|SetIntensity _pointlight (Variables|Default|GetLight%20Intensity))
  (Rendering|Lighting|SetAttenuationRadius _pointlight (Variables|Default|GetLight%20Radius))
  (if (Variables|Default|GetLight%20Uses%20Temperature)
    (Class|LightComponent|SetTemperature _pointlight (Variables|Default|GetLight%20Temperature))
    (else
      (Rendering|Components|Light|SetLightColor _pointlight (Variables|Default|GetLight%20Color) true)))
  (if (Variables|Default|GetRandomize%20Candle%20By%20Position)
    (switch int (Math|Random|RandomIntegerinRangefromStream (Math|Random|MakeRandomStream (Math|Float|Truncate (+ (+ _x _y) _z))) 0 9)
      (:Default
        (Components|StaticMesh|SetStaticMesh _candle_2 "/Game/Vefects/Candle_VFX/VFX/Candle_Melted/SM/SM_Melted_Candle_01.SM_Melted_Candle_01" :!label _label)
        (Variables|Default|SetWick%20Vertical%20Position 0.5)
        (Class|KismetMathLibrary|VectorSet _flame_position 1.26 -1.13 5.55))
      (:0
        (goto _label))
      (:1
        (Components|StaticMesh|SetStaticMesh _candle_2 "/Game/Vefects/Candle_VFX/VFX/Candle_Melted/SM/SM_Melted_Candle_02.SM_Melted_Candle_02" :!label _label_2)
        (Variables|Default|SetWick%20Vertical%20Position 0.96)
        (Class|KismetMathLibrary|VectorSet _flame_position 0.0 0.0 11.0))
      (:2
        (Components|StaticMesh|SetStaticMesh _candle_2 "/Game/Vefects/Candle_VFX/VFX/Candle_Melted/SM/SM_Melted_Candle_03.SM_Melted_Candle_03" :!label _label_3)
        (Variables|Default|SetWick%20Vertical%20Position 0.96)
        (Class|KismetMathLibrary|VectorSet _flame_position 0.0 0.0 11.0))
      (:3
        (Components|StaticMesh|SetStaticMesh _candle_2 "/Game/Vefects/Candle_VFX/VFX/Candle_Melted/SM/SM_Melted_Candle_04.SM_Melted_Candle_04" :!label _label_4)
        (Variables|Default|SetWick%20Vertical%20Position 0.55)
        (Class|KismetMathLibrary|VectorSet _flame_position 0.5 0.0 6.6))
      (:4
        (Components|StaticMesh|SetStaticMesh _candle_2 "/Game/Vefects/Candle_VFX/VFX/Candle_Melted/SM/SM_Melted_Candle_05.SM_Melted_Candle_05" :!label _label_5)
        (Variables|Default|SetWick%20Vertical%20Position 0.5)
        (Class|KismetMathLibrary|VectorSet _flame_position 0.6 0.5 5.5))
      (:5
        (Components|StaticMesh|SetStaticMesh _candle_2 "/Game/Vefects/Candle_VFX/VFX/Candle_Glass/SM/SM_VFX_Archviz_Candle_Glass_01.SM_VFX_Archviz_Candle_Glass_01" :!label _label_6)
        (Variables|Default|SetWick%20Vertical%20Position 0.96)
        (Class|KismetMathLibrary|VectorSet _flame_position 0.0 0.0 10.5))
      (:6
        (Components|StaticMesh|SetStaticMesh _candle_2 "/Game/Vefects/Candle_VFX/VFX/Candle_Glass/SM/SM_VFX_Archviz_Candle_Glass_01_VC.SM_VFX_Archviz_Candle_Glass_01_VC" :!label _label_7)
        (Variables|Default|SetWick%20Vertical%20Position 0.96)
        (Class|KismetMathLibrary|VectorSet _flame_position 0.0 0.0 10.5))
      (:7
        (Components|StaticMesh|SetStaticMesh _candle_2 "/Game/Vefects/Candle_VFX/VFX/Candle_Glass/SM/SM_VFX_Archviz_Candle_Glass_02_VC.SM_VFX_Archviz_Candle_Glass_02_VC" :!label _label_8)
        (Variables|Default|SetWick%20Vertical%20Position 0.96)
        (Class|KismetMathLibrary|VectorSet _flame_position 0.0 0.0 10.5))
      (:8
        (Components|StaticMesh|SetStaticMesh _candle_2 "/Game/Vefects/Candle_VFX/VFX/Candle_Sphere_Cube/SM/SM_VFX_Archviz_Candle_Sphere_Cube_01.SM_VFX_Archviz_Candle_Sphere_Cube_01" :!label _label_9)
        (Variables|Default|SetWick%20Vertical%20Position 0.96)
        (Class|KismetMathLibrary|VectorSet _flame_position 0.0 0.0 10.5))
      (:9
        (Components|StaticMesh|SetStaticMesh _candle_2 "/Game/Vefects/Candle_VFX/VFX/Candle_Cloud/SM/SM_VFX_Archviz_Candle_Cloud_01.SM_VFX_Archviz_Candle_Cloud_01" :!label _label_10)
        (Variables|Default|SetWick%20Vertical%20Position 0.85)
        (Class|KismetMathLibrary|VectorSet _flame_position 0.0 0.0 4.8)))
    (else
      (switch int (Variables|Default|GetCandle%20Type)
        (:Default
          (goto _label))
        (:0
          (goto _label))
        (:1
          (goto _label_2))
        (:2
          (goto _label_3))
        (:3
          (goto _label_4))
        (:4
          (goto _label_5))
        (:5
          (goto _label_6))
        (:6
          (goto _label_7))
        (:7
          (goto _label_8))
        (:8
          (goto _label_9))
        (:9
          (goto _label_10)))))
  (Transformation|SetRelativeLocation (Variables|Default|GetFlamesSmokePosition) (+ (Variables|Default|GetFlame%20Position) (Variables|Default|GetFlame%20Position%20Offset)) false false)
  (if (Variables|Default|GetCandle%20Wax%20Custom%20Color)
    (bind _returnvalue_2 (Rendering|Material|CreateDynamicMaterialInstance (Variables|Default|GetCandle) 0 "/Game/Vefects/Candle_VFX/Shared/Materials/Burley/MI_Candle_SSSB_VC_Colored_Scent_BP_01.MI_Candle_SSSB_VC_Colored_Scent_BP_01" "None" :!class /Script/Engine.PrimitiveComponent))
    (Variables|Default|SetWaxCustomColorMat _returnvalue_2)
    (Rendering|Material|SetVectorParameterValue (Variables|Default|GetWaxCustomColorMat) "Color 01" (Variables|Default|GetCandle%20Wax%20Color) :!class /Script/Engine.MaterialInstanceDynamic)
    (else
      (switch int (Variables|Default|GetCandle%20Color)
        (:Default
          (Rendering|Material|SetMaterial _candle_3 0 "/Game/Vefects/Candle_VFX/Shared/Materials/Burley/MI_Candle_SSS_Profile_Burley_VC_01.MI_Candle_SSS_Profile_Burley_VC_01" :!label _label_11))
        (:0
          (goto _label_11))
        (:1
          (Rendering|Material|SetMaterial _candle_3 0 "/Game/Vefects/Candle_VFX/Shared/Materials/Burley/MI_Candle_SSSB_VC_Colored_Scent_01.MI_Candle_SSSB_VC_Colored_Scent_01"))
        (:2
          (Rendering|Material|SetMaterial _candle_3 0 "/Game/Vefects/Candle_VFX/Shared/Materials/Burley/MI_Candle_SSSB_VC_Colored_Scent_02.MI_Candle_SSSB_VC_Colored_Scent_02"))
        (:3
          (Rendering|Material|SetMaterial _candle_3 0 "/Game/Vefects/Candle_VFX/Shared/Materials/Burley/MI_Candle_SSSB_VC_Colored_Scent_03.MI_Candle_SSSB_VC_Colored_Scent_03"))
        (:4
          (Rendering|Material|SetMaterial _candle_3 0 "/Game/Vefects/Candle_VFX/Shared/Materials/Burley/MI_Candle_SSSB_VC_Colored_Scent_04.MI_Candle_SSSB_VC_Colored_Scent_04"))
        (:5
          (Rendering|Material|SetMaterial _candle_3 0 "/Game/Vefects/Candle_VFX/Shared/Materials/Burley/MI_Candle_SSSB_VC_Colored_Scent_05.MI_Candle_SSSB_VC_Colored_Scent_05"))
        (:6
          (Rendering|Material|SetMaterial _candle_3 0 "/Game/Vefects/Candle_VFX/Shared/Materials/Burley/MI_Candle_SSSB_VC_Colored_Scent_06.MI_Candle_SSSB_VC_Colored_Scent_06"))
        (:7
          (Rendering|Material|SetMaterial _candle_3 0 "/Game/Vefects/Candle_VFX/Shared/Materials/Burley/MI_Candle_SSSB_VC_Colored_Scent_07.MI_Candle_SSSB_VC_Colored_Scent_07"))
        (:8
          (Rendering|Material|SetMaterial _candle_3 0 "/Game/Vefects/Candle_VFX/Shared/Materials/Burley/MI_Candle_SSSB_VC_Colored_Scent_08.MI_Candle_SSSB_VC_Colored_Scent_08"))
        (:9
          (Rendering|Material|SetMaterial _candle_3 0 "/Game/Vefects/Candle_VFX/Shared/Materials/Burley/MI_Candle_SSSB_VC_Colored_Scent_09.MI_Candle_SSSB_VC_Colored_Scent_09"))
        (:10
          (Rendering|Material|SetMaterial _candle_3 0 "/Game/Vefects/Candle_VFX/Shared/Materials/Burley/MI_Candle_SSSB_VC_Colored_Scent_10.MI_Candle_SSSB_VC_Colored_Scent_10"))
        (:11
          (Rendering|Material|SetMaterial _candle_3 0 "/Game/Vefects/Candle_VFX/Shared/Materials/Burley/MI_Candle_SSSB_VC_Colored_Scent_11.MI_Candle_SSSB_VC_Colored_Scent_11"))
        (:12
          (Rendering|Material|SetMaterial _candle_3 0 "/Game/Vefects/Candle_VFX/Shared/Materials/Burley/MI_Candle_SSSB_VC_Colored_Scent_12.MI_Candle_SSSB_VC_Colored_Scent_12"))
        (:13
          (Rendering|Material|SetMaterial _candle_3 0 "/Game/Vefects/Candle_VFX/Shared/Materials/Burley/MI_Candle_SSSB_VC_Colored_Scent_13.MI_Candle_SSSB_VC_Colored_Scent_13"))
        (:14
          (Rendering|Material|SetMaterial _candle_3 0 "/Game/Vefects/Candle_VFX/Shared/Materials/Burley/MI_Candle_SSSB_VC_Colored_Scent_14.MI_Candle_SSSB_VC_Colored_Scent_14"))
        (:15
          (Rendering|Material|SetMaterial _candle_3 0 "/Game/Vefects/Candle_VFX/Shared/Materials/Burley/MI_Candle_SSSB_VC_Colored_Scent_15.MI_Candle_SSSB_VC_Colored_Scent_15"))
        (:16
          (Rendering|Material|SetMaterial _candle_3 0 "/Game/Vefects/Candle_VFX/Shared/Materials/Burley/MI_Candle_SSSB_VC_Colored_Scent_16.MI_Candle_SSSB_VC_Colored_Scent_16")))))
  (if (Variables|Default|GetLit%20Wick)
    (bind _returnvalue_3 (Rendering|Material|CreateDynamicMaterialInstance _candle 1 "/Game/Vefects/Candle_VFX/Shared/Materials/Wick/MI_Candle_Wick_BP_01.MI_Candle_Wick_BP_01" "None" :!class /Script/Engine.PrimitiveComponent))
    (Variables|Default|SetWickMaterial _returnvalue_3)
    (Rendering|Material|SetScalarParameterValue (Variables|Default|GetWickMaterial) "Emissive Multiply" (Variables|Default|GetWick%20Emissive) :!class /Script/Engine.MaterialInstanceDynamic)
    (Rendering|Material|SetVectorParameterValue (Variables|Default|GetWickMaterial) "Color Tip" (Variables|Default|GetWick%20Color) :!class /Script/Engine.MaterialInstanceDynamic)
    (Rendering|Material|SetScalarParameterValue (Variables|Default|GetWickMaterial) "Burning Tip Vertical Position" (+ (Variables|Default|GetWick%20Vertical%20Position%20Offset) (Variables|Default|GetWick%20Vertical%20Position)) :!class /Script/Engine.MaterialInstanceDynamic)
    (Rendering|Material|SetScalarParameterValue (Variables|Default|GetWickMaterial) "Burning Tip Falloff" (Variables|Default|GetWick%20Falloff) :!class /Script/Engine.MaterialInstanceDynamic)
    (Rendering|Material|SetMaterial _candle 1 (Variables|Default|GetWickMaterial))
    (else
      (Rendering|Material|SetMaterial (Variables|Default|GetCandle) 1 "/Game/Vefects/Candle_VFX/Shared/Materials/Wick/MI_Candle_Wick_Off_01.MI_Candle_Wick_Off_01"))))