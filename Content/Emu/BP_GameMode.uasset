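; VR game mode that runs the game's flow as a Menu, Playing, Paused, Win and Lose state machine, starting from the game instance's next initial state.
; Non-playing states lock pawn movement and spawn their panel level in front of the camera, facing it.
; They near-freeze global time, offsetting it with the pawn's custom dilation.
; Checkpoint notifications trigger nothing yet, and both set the stone-circle flag.
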(event Custom|EnterMenuState
  (bind _playerpawn (Variables|Default|GetPlayerPawn))
  (Utilities|FlowControl|Delay 0.1)
  (Default|EndTeleportTrace _playerpawn)
  (Variables|/Game/XRFramework/Blueprints/BP_XRPawn.BP_XRPawn_C|SetbMovementEnabled _playerpawn false)
  (bind _spawntransform (CallFunction|CalculateSpawnTransform (Variables|/Game/XRFramework/Blueprints/BP_XRPawn.BP_XRPawn_C|GetCamera _playerpawn)))
  (bind _returnvalue (Game|SpawnActorfromClass "/Game/Emu/HUD/MainMenu/BP_MenuPanel.BP_MenuPanel_C" _spawntransform "Undefined" "MultiplyWithRoot" 0 0))
  (Variables|Default|SetMenuPanelRef _returnvalue)
  (CallFunction|SetTimeDilation 0.001 1e+03))

(event Custom|EnterPlayingState
  (bind _menupanelref (Variables|Default|GetMenuPanelRef))
  (bind _playerpawn (Variables|Default|GetPlayerPawn))
  (bind _pausepanelref (Variables|Default|GetPausePanelRef))
  (Default|EndTeleportTrace _playerpawn)
  (Variables|/Game/XRFramework/Blueprints/BP_XRPawn.BP_XRPawn_C|SetbMovementEnabled _playerpawn true)
  (if (Utilities|IsValid _menupanelref)
    (Actor|DestroyActor _menupanelref))
  (if (Utilities|IsValid _pausepanelref)
    (Actor|DestroyActor _pausepanelref))
  (Default|HUDVisibilityToggle (Variables|Default|GetPlayerPawn) true)
  (CallFunction|SetTimeDilation 1.0 1.0))

(event Custom|EnterPausedState
  (bind _playerpawn (Variables|Default|GetPlayerPawn))
  (Default|EndTeleportTrace _playerpawn)
  (Variables|/Game/XRFramework/Blueprints/BP_XRPawn.BP_XRPawn_C|SetbMovementEnabled _playerpawn false)
  (bind _spawntransform (CallFunction|CalculateSpawnTransform (Variables|/Game/XRFramework/Blueprints/BP_XRPawn.BP_XRPawn_C|GetCamera _playerpawn)))
  (bind _returnvalue (Game|SpawnActorfromClass "/Game/Emu/HUD/PauseMenu/BP_PausePanel.BP_PausePanel_C" _spawntransform "Undefined" "MultiplyWithRoot" 0 0))
  (Variables|Default|SetPausePanelRef _returnvalue)
  (Default|HUDVisibilityToggle (Variables|Default|GetPlayerPawn) false)
  (CallFunction|SetTimeDilation 0.001 1e+03))

(event Custom|EnterWinState
  (bind _playerpawn (Variables|Default|GetPlayerPawn))
  (Default|EndTeleportTrace _playerpawn)
  (Variables|/Game/XRFramework/Blueprints/BP_XRPawn.BP_XRPawn_C|SetbMovementEnabled _playerpawn false)
  (bind _spawntransform (CallFunction|CalculateSpawnTransform (Variables|/Game/XRFramework/Blueprints/BP_XRPawn.BP_XRPawn_C|GetCamera _playerpawn)))
  (Game|SpawnActorfromClass "/Game/Emu/HUD/Win/BP_WinPanel.BP_WinPanel_C" _spawntransform "Undefined" "MultiplyWithRoot" 0 0)
  (CallFunction|SetTimeDilation 0.001 1e+03))

(event Custom|EnterLoseState
  (bind _playerpawn (Variables|Default|GetPlayerPawn))
  (Default|EndTeleportTrace _playerpawn)
  (Variables|/Game/XRFramework/Blueprints/BP_XRPawn.BP_XRPawn_C|SetbMovementEnabled _playerpawn false)
  (bind _spawntransform (CallFunction|CalculateSpawnTransform (Variables|/Game/XRFramework/Blueprints/BP_XRPawn.BP_XRPawn_C|GetCamera _playerpawn)))
  (Game|SpawnActorfromClass "/Game/Emu/HUD/Lose/BP_LosePanel.BP_LosePanel_C" _spawntransform "Undefined" "MultiplyWithRoot" 0 0)
  (CallFunction|SetTimeDilation 0.001 1e+03)
  (bind _outactors (Actor|GetAllActorsOfClass 0))
  (Actor|DestroyActor (Utilities|Array|Get(acopy) _outactors)))

(event EventBeginPlay
  (bind _asbp_xrpawn (Utilities|Casting|CastToBP_XRPawn (Game|Player|GetPlayerPawn 0)))
  (Variables|Default|SetPlayerPawn _asbp_xrpawn)
  (bind _asbp_game_instance (Utilities|Casting|CastToBP_GameInstance (Game|GetGameInstance)))
  (CallFunction|SetFlowState (Variables|/Game/Emu/BP_GameInstance.BP_GameInstance_C|GetNextInitialState _asbp_game_instance)))

(fn ConstructionScript)

(fn SetFlowState
  (params (NewState :type E_GameFlowState%20Enum :default "NewEnumerator0"))
  (bind _output_get (Variables|Default|SetFlowState NewState))
  (switch Utilities|FlowControl|Switch|SwitchonE_GameFlowState _output_get
    (:NewEnumerator0
      (CallFunction|EnterMenuState))
    (:NewEnumerator1
      (CallFunction|EnterPlayingState))
    (:NewEnumerator2
      (CallFunction|EnterPausedState))
    (:NewEnumerator3
      (CallFunction|EnterWinState))
    (:NewEnumerator4
      (CallFunction|EnterLoseState))))

(fn CalculateSpawnTransform
  (params (Camera :type Camera%20Component%20Object%20Reference))
  (bind _returnvalue (Transformation|GetWorldLocation Camera))
  (bind _returnvalue_2 (Math|Vector|GetForwardVector Camera))
  (bind _distance (Variables|Default|GetDistance))
  (bind _heightoffset (Variables|Default|GetHeightOffset))
  (bind _returnvalue_3 (Math|Vector|MakeVector (.x _returnvalue_2) (.y _returnvalue_2) 0.0))
  (bind _returnvalue_4 (Math|Vector|Normalize _returnvalue_3))
  (bind _returnvalue_5 (* _distance _returnvalue_4))
  (bind _returnvalue_6 (+ _returnvalue_5 _returnvalue))
  (bind _returnvalue_7 (+ (.z _returnvalue_6) _heightoffset))
  (bind _returnvalue_8 (Math|Vector|MakeVector (.x _returnvalue_6) (.y _returnvalue_6) _returnvalue_7))
  (return (Math|Transform|MakeTransform _returnvalue_8 (Math|Rotator|MakeRotator 0.0 0.0 (.yaw (Math|Rotator|FindLookatRotation _returnvalue_8 _returnvalue))))))

(fn SetTimeDilation
  (params (GlobalTimeDilation :type Float%20%28double-precision%29) (PlayerTimeDilation :type Float%20%28double-precision%29))
  (Utilities|Time|SetGlobalTimeDilation GlobalTimeDilation)
  (Variables|/Script/Engine.Actor|SetCustomTimeDilation (Variables|Default|GetPlayerPawn) PlayerTimeDilation))

(fn NotifyCheckpointCompleted
  (params (Checkpoint%20Type :type E_CheckpointType%20Enum :default "E_CheckpointType_MAX"))
  (switch Utilities|FlowControl|Switch|SwitchonE_CheckpointType Checkpoint%20Type
    (:NewEnumerator0
      (Variables|Default|SetbStoneCircleCompleted true)
      (if (Variables|Default|GetbStoneCircleCompleted)
        _))
    (:NewEnumerator1
      (Variables|Default|SetbStoneCircleCompleted true)
      (if (Variables|Default|GetbCandleRitualCompleted)
        _))))