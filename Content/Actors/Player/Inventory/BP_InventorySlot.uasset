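; Inventory slot actor that holds one grabbable object of an accepted class, snapped to itself.
; Overlapping AcceptanceRange binds the object's BP_GrabComponent grab and drop events and previews its mesh with an overlay material; leaving unbinds and clears it.
; Dropping in range disables physics and attaches the object if the slot is empty.
; Grabbing the held object detaches it and frees the slot.
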(event OnComponentBeginOverlap(AcceptanceRange)
  (params (OverlappedComponent :type Primitive%20Component%20Object%20Reference) (OtherActor :type Actor%20Object%20Reference) (OtherComp :type Primitive%20Component%20Object%20Reference) (OtherBodyIndex :type Integer) (bFromSweep :type Boolean) (SweepResult :type Hit%20Result%20Structure%20%28by%20ref%29))
  (bind _returnvalue (Actor|GetComponentsByClass OtherActor "/Game/XRFramework/Blueprints/BP_GrabComponent.BP_GrabComponent_C"))
  (if (and (Utilities|Set|Contains (Variables|Default|GetAcceptedObjects) (Utilities|GetClass OtherActor)) (Utilities|Array|IsNotEmpty _returnvalue))
    (for _array_element _returnvalue
      (Utilities|Array|Add (Variables|Default|GetTackedComponents) _array_element)
      (EventDispatchers|AssignOnGrabbed _array_element (delegate Custom|OnGrabbed_Event))
      (EventDispatchers|AssignOnDropped _array_element (delegate Custom|OnDropped_Event)))
    (CallFunction|CreatePlacementHelper (Actor|GetComponentbyClass OtherActor "/Script/Engine.StaticMeshComponent"))))

(event OnComponentEndOverlap(AcceptanceRange)
  (params (OverlappedComponent :type Primitive%20Component%20Object%20Reference) (OtherActor :type Actor%20Object%20Reference) (OtherComp :type Primitive%20Component%20Object%20Reference) (OtherBodyIndex :type Integer))
  (bind _returnvalue (Actor|GetComponentsByClass OtherActor "/Game/XRFramework/Blueprints/BP_GrabComponent.BP_GrabComponent_C"))
  (if (Utilities|Array|IsNotEmpty _returnvalue)
    (for _array_element _returnvalue
      (Utilities|Array|RemoveItem (Variables|Default|GetTackedComponents) _array_element)
      (EventDispatchers|UnbindEventfromOnGrabbed _array_element (delegate Custom|OnGrabbed_Event))
      (EventDispatchers|UnbindEventfromOnDropped _array_element (delegate Custom|OnDropped_Event))
      (CallFunction|DestroyPlacementHelper))))

(event Custom|OnGrabbed_Event
  (params (Self%20Reference :type BP%20Grab%20Component%20Object%20Reference))
  (CallFunction|TryDrop (Components|GetOwner Self%20Reference)))

(event Custom|OnDropped_Event
  (params (Self%20Reference :type BP%20Grab%20Component%20Object%20Reference))
  (CallFunction|TryAttach Self%20Reference))

(event EventBeginPlay)

(event Collision|EventActorBeginOverlap
  (params (OtherActor :type Actor%20Object%20Reference)))

(event EventTick
  (params (DeltaSeconds :type Float%20%28single-precision%29)))

(fn ConstructionScript)

(fn TryAttach
  (params (Grab%20Component :type BP%20Grab%20Component%20Object%20Reference))
  (Utilities|IsValid (Variables|Default|GetHeldActor) ; Check if anything in the slot already
    (:Is%20Not%20Valid
      (bind _output_get (Variables|Default|SetHeldActor (Components|GetOwner Grab%20Component)))
      (Default|SetPrimitiveCompPhysics Grab%20Component false)
      (Transformation|AttachActorToActor _output_get self "None" "SnapToTarget" "SnapToTarget" "KeepRelative" false))))

(fn TryDrop
  (params (Actor :type Actor%20Object%20Reference))
  (Utilities|IsValid (Variables|Default|GetHeldActor)
    (:Is%20Valid
      (if (== 0 (Variables|Default|GetHeldActor))
        (if (== (Actor|GetAttachParentActor (Variables|Default|GetHeldActor)) self)
          (Transformation|DetachFromActor (Variables|Default|GetHeldActor) "KeepRelative" "KeepRelative" "KeepRelative"))
        (Variables|Default|SetHeldActor 0)))))

(fn CreatePlacementHelper
  (params (StaticMesh :type Static%20Mesh%20Component%20Object%20Reference))
  (bind _placementhelper (Variables|Default|GetPlacementHelper))
  (Utilities|IsValid StaticMesh
    (:Is%20Valid
      (Components|StaticMesh|SetStaticMesh _placementhelper (Variables|/Script/Engine.StaticMeshComponent|GetStaticMesh StaticMesh))
      (Transformation|SetWorldScale3D _placementhelper (Transformation|GetWorldScale StaticMesh))
      (Rendering|Material|SetMaterial _placementhelper 0 "/Game/Actors/Player/Inventory/M_OverlayMaterial.M_OverlayMaterial"))))

(fn DestroyPlacementHelper
  (Components|StaticMesh|SetStaticMesh (Variables|Default|GetPlacementHelper) 0))